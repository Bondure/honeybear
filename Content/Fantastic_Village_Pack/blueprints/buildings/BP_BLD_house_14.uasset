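; Windmill house building that acts as a central honey store, tallying honey for five bee types.
; Tick nudges the sail's pitch by a fixed, frame-dependent step with a reset at 90 degrees, and refreshes each type's count text.
; The add_hony event sweeps all Bpac_build actors, moving each type's honey into its own map and zeroing the source, skipping transfers that would exceed the 100 cap.
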(event `self.ReceiveTick`
  (params (DeltaSeconds :type "Float (single-precision)"))
  (bind _quanity_honey (`self.Quanity Honey`))
  (bind _sm_bld_windmill_sail (`self.SM_BLD_windmill_sail`))
  (bind (_relativerotation_roll _relativerotation_pitch) (`KismetMathLibrary.BreakRotator` (`SceneComponent.RelativeRotation` _sm_bld_windmill_sail)))
  (`|ExecutionSequence`
    (:`then_0`
      (if (== _relativerotation_pitch 90.0)
        (`SceneComponent.K2_SetRelativeRotation` _sm_bld_windmill_sail (`KismetMathLibrary.MakeRotator` 0.0 0.0 -180.0) false false)
        (else
          (`SceneComponent.K2_SetRelativeRotation` (`self.SM_BLD_windmill_sail`) (`KismetMathLibrary.MakeRotator` 0.0 (+ _relativerotation_pitch 0.05) -180.0) false false))))
    (:`then_1`
      (`TextRenderComponent.K2_SetText` (`self.normal`) (`KismetTextLibrary.Conv_IntToText` (`BlueprintMapLibrary.Map_Find` _quanity_honey "/Game/blueprints/bpchar_bee.bpchar_bee_C")))
      (`TextRenderComponent.K2_SetText` (`self.lava`) (`KismetTextLibrary.Conv_IntToText` (`BlueprintMapLibrary.Map_Find` _quanity_honey "/Game/blueprints/BPchar_lava_bee.BPchar_lava_bee_C")))
      (`TextRenderComponent.K2_SetText` (`self.rock`) (`KismetTextLibrary.Conv_IntToText` (`BlueprintMapLibrary.Map_Find` _quanity_honey "/Game/blueprints/bpchar_bee_rock.bpchar_bee_rock_C")))
      (`TextRenderComponent.K2_SetText` (`self.ice`) (`KismetTextLibrary.Conv_IntToText` (`BlueprintMapLibrary.Map_Find` _quanity_honey "/Game/blueprints/bpchar_bee_ice.bpchar_bee_ice_C")))
      (`TextRenderComponent.K2_SetText` (`self.cat`) (`KismetTextLibrary.Conv_IntToText` (`BlueprintMapLibrary.Map_Find` _quanity_honey "/Game/blueprints/bpchar_bee_cat.bpchar_bee_cat_C"))))))

(event `add_hony`
  (bind _quanity_honey (`self.Quanity Honey`))
  (bind _outactors (`GameplayStatics.GetAllActorsOfClass` "/Game/blueprints/bpac_build.bpac_build_C"))
  (for _array_element _outactors
    (bind _asbpac_build (cast `/Game/blueprints/bpac_build` _array_element))
    (for _array_element_2 (`/Game/blueprints/bpac_build.classarray` _asbpac_build)
      (bind _quanity_honey_2 (`/Game/blueprints/bpac_build.quanity_honey` _asbpac_build))
      (bind _returnvalue (+ (`BlueprintMapLibrary.Map_Find` _quanity_honey _array_element_2) (`BlueprintMapLibrary.Map_Find` _quanity_honey_2 _array_element_2)))
      (if (< _returnvalue 101)
        (`BlueprintMapLibrary.Map_Add` _quanity_honey _array_element_2 _returnvalue)
        (`BlueprintMapLibrary.Map_Add` _quanity_honey_2 _array_element_2)))))

(fn `UserConstructionScript`)