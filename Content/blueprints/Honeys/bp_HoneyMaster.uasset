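; Honey pickup actor that picks a random honey type at BeginPlay, shows a rock mesh and goes into the first-person character's inventory on box overlap.
; The honey's class display name keys parallel name and count arrays on the character: a match stacks up to 10, otherwise it takes an empty slot.
; DoOnce guards each successful pickup before the actor destroys itself; otherwise it stays in the world.
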(event `self.ReceiveBeginPlay`
  (set `self.Hon` (`KismetArrayLibrary.Array_Random` (`self.Random Honey`)))
  (`StaticMeshComponent.SetStaticMesh` (`self.StaticMesh`) "/Game/InfinityBladeFireLands/Environments/Fire/Fire_Fortress/SM/Env_Fire_NordRock01.Env_Fire_NordRock01"))

(event `self.Box.OnComponentBeginOverlap`
  (params (OverlappedComponent :type "PrimitiveComponent Object Reference") (OtherActor :type "Actor Object Reference") (OtherComp :type "PrimitiveComponent Object Reference") (OtherBodyIndex :type Integer) (bFromSweep :type Boolean) (SweepResult :type "HitResult Structure (by ref)"))
  (bind _hon (`self.Hon`))
  (bind _asbp_first_person_character (cast `/Game/FirstPerson/Blueprints/BP_FirstPersonCharacter` OtherActor))
  (bind _str_name_of_bee_inventory (`/Game/FirstPerson/Blueprints/BP_FirstPersonCharacter.str_name_of_bee_inventory` _asbp_first_person_character))
  (bind _returnvalue (`KismetArrayLibrary.Array_Find` _str_name_of_bee_inventory))
  (if (== _returnvalue -1)
    (bind _returnvalue_2 (`KismetArrayLibrary.Array_Find` _str_name_of_bee_inventory (`KismetSystemLibrary.GetClassDisplayName` _hon)))
    (bind _returnvalue_3 (== _returnvalue_2 -1))
    (if (not _returnvalue_3) :!label _label
      (bind _int_conunt_of_honey_inventory (`/Game/FirstPerson/Blueprints/BP_FirstPersonCharacter.int_conunt_of_honey_inventory` _asbp_first_person_character))
      (bind _output (`|GetArrayItem` _int_conunt_of_honey_inventory _returnvalue_2))
      (if (!= _output 10)
        (`/Engine/EditorBlueprintResources/StandardMacros.DoOnce` false
          (:`Completed`
            (`KismetArrayLibrary.Array_Set` _int_conunt_of_honey_inventory _returnvalue_2 (+ _output 1))
            (`self.K2_DestroyActor`)))))
    (elif _returnvalue_3
      (`/Engine/EditorBlueprintResources/StandardMacros.DoOnce` false
        (:`Completed`
          (`KismetArrayLibrary.Array_Set` _int_conunt_of_honey_inventory _returnvalue 1)
          (`KismetArrayLibrary.Array_Set` _str_name_of_bee_inventory _returnvalue (`KismetSystemLibrary.GetClassDisplayName` _hon))
          (`KismetSystemLibrary.Delay` 0.1)
          (`self.K2_DestroyActor`)))
      (else
        (goto _label)))))

(fn `UserConstructionScript`)