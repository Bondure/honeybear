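; Mob character logic that wanders, chases the player on detection and deals timed damage in attack range.
; Overlap spheres set hearing and attack states, which Tick turns into AI moves or HP loss, with a ten-second stun pausing both.
; Leaving the optimization sphere, or a player DeltaSeconds check at BeginPlay, swaps the mob for an OptimizeActor storing its class and transform.
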(event `self.ReceiveBeginPlay`
  (bind _asbp_first_person_character (cast `/Game/FirstPerson/Blueprints/BP_FirstPersonCharacter` (`GameplayStatics.GetPlayerPawn` 0)))
  (set `CharacterMovementComponent.RotationRate` (`KismetMathLibrary.MakeRotator` 360.0 (`self.float_rotation_speed`) 360.0) (`self.CharacterMovement`))
  (if (< (`/Game/FirstPerson/Blueprints/BP_FirstPersonCharacter.Delta Seconds` _asbp_first_person_character) 30.0)
    (`self.SpawnOptimize`)))

(event `self.ReceiveTick`
  (params (DeltaSeconds :type "Float (single-precision)"))
  (bind _mob_to_go (`self.mob_to_go`))
  (bind _timer (`self.timer`))
  (bind _charactermovement (`self.CharacterMovement`))
  (`|ExecutionSequence`
    (:`then_0`
      (if (`self.bool_stan`)
        (bind _output_get (set `self.timer` (+ (`self.timer`) DeltaSeconds)))
        (if (> _output_get 10.0)
          (set `self.bool_stan` false)
          (set `self.timer` 0.0))
        (else
          (set `self.timer` (+ _timer DeltaSeconds))
          (if (`self.bool_player_in_atack`)
            (if (> (`self.timer`) (`self.float_attack_speed`))
              (bind _asbp_first_person_character (cast `/Game/FirstPerson/Blueprints/BP_FirstPersonCharacter` _mob_to_go)
                (:`then`
                  (set `/Game/FirstPerson/Blueprints/BP_FirstPersonCharacter.float_hp` (- (`/Game/FirstPerson/Blueprints/BP_FirstPersonCharacter.float_hp` _asbp_first_person_character) (`self.float_damage`)) _asbp_first_person_character)
                  (set `self.timer` 0.0))
                (:`CastFailed`
                  (cast `/Game/blueprints/bpchar_bee` _mob_to_go))))
            (elif (`self.bool_hear`)
              (set `CharacterMovementComponent.MaxWalkSpeed` (`self.float_run_speed`) _charactermovement)
              (`AIController.MoveToActor` (`AIBlueprintHelperLibrary.GetAIController` self) (`self.mob_to_go`) (`self.float_attack_radius`) true true true null true)
              (else
                (set `CharacterMovementComponent.MaxWalkSpeed` (`self.float_walk_speed`) _charactermovement)
                (if (> _timer (* (`KismetMathLibrary.RandomFloat`) 100.0))
                  (if true
                    (set `self.timer` 0.0)
                    (bind _randomlocation (`NavigationSystemV1.K2_GetRandomLocationInNavigableRadius` (`SceneComponent.K2_GetComponentLocation` (`self.CapsuleComponent`)) 1000.0 null null))
                    (`AIController.MoveToLocation` (`AIBlueprintHelperLibrary.GetAIController` self) (`KismetMathLibrary.MakeVector` (.x _randomlocation) (.y _randomlocation) (.z _randomlocation)) -1.0 true false false true null true)))))))))))

(event `self.Sphere.OnComponentBeginOverlap`
  (params (OverlappedComponent :type "PrimitiveComponent Object Reference") (OtherActor :type "Actor Object Reference") (OtherComp :type "PrimitiveComponent Object Reference") (OtherBodyIndex :type Integer) (bFromSweep :type Boolean) (SweepResult :type "HitResult Structure (by ref)"))
  ;[1 1 1] атака  тригер
  (`|ExecutionSequence`
    (:`then_0`
      (cast `/Game/FirstPerson/Blueprints/BP_FirstPersonCharacter` OtherActor)
      (set `self.bool_player_in_atack` true)
      (set `self.bool_hear` false)
      (set `self.mob_to_go` OtherActor))))

(event `self.Sphere.OnComponentEndOverlap`
  (params (OverlappedComponent :type "PrimitiveComponent Object Reference") (OtherActor :type "Actor Object Reference") (OtherComp :type "PrimitiveComponent Object Reference") (OtherBodyIndex :type Integer))
  ;[1 1 1] атака  тригер
  (`|ExecutionSequence`
    (:`then_0`
      (cast `/Game/FirstPerson/Blueprints/BP_FirstPersonCharacter` OtherActor)
      (set `self.bool_player_in_atack` false)
      (set `self.bool_hear` true))))

(event `self.Sphere1.OnComponentBeginOverlap`
  (params (OverlappedComponent :type "PrimitiveComponent Object Reference") (OtherActor :type "Actor Object Reference") (OtherComp :type "PrimitiveComponent Object Reference") (OtherBodyIndex :type Integer) (bFromSweep :type Boolean) (SweepResult :type "HitResult Structure (by ref)"))
  ;[1 1 1] тригер слуха
  (`|ExecutionSequence`
    (:`then_0`
      (cast `/Game/FirstPerson/Blueprints/BP_FirstPersonCharacter` OtherActor)
      (set `self.bool_hear` true)
      (set `self.mob_to_go` OtherActor))))

(event `self.Sphere1.OnComponentEndOverlap`
  (params (OverlappedComponent :type "PrimitiveComponent Object Reference") (OtherActor :type "Actor Object Reference") (OtherComp :type "PrimitiveComponent Object Reference") (OtherBodyIndex :type Integer))
  ;[1 1 1] тригер слуха
  (`|ExecutionSequence`
    (:`then_0`
      (cast `/Game/FirstPerson/Blueprints/BP_FirstPersonCharacter` OtherActor)
      (set `self.bool_hear` false))))

(event `self.SphereforOptimization.OnComponentEndOverlap`
  (params (OverlappedComponent :type "PrimitiveComponent Object Reference") (OtherActor :type "Actor Object Reference") (OtherComp :type "PrimitiveComponent Object Reference") (OtherBodyIndex :type Integer))
  (cast `/Game/FirstPerson/Blueprints/BP_FirstPersonCharacter` OtherActor)
  (`/Engine/EditorBlueprintResources/StandardMacros.DoOnce` false
    (:`Completed`
      (`self.SpawnOptimize`))))

(event `SpawnOptimize`
  (bind _returnvalue (`self.GetTransform` self))
  (`|SpawnActorFromClass` "/Game/blueprints/OptimizeActor.OptimizeActor_C" _returnvalue "AlwaysSpawn" "MultiplyWithRoot" null (`GameplayStatics.GetObjectClass` self) _returnvalue null)
  (`self.K2_DestroyActor`))

(fn `UserConstructionScript`)