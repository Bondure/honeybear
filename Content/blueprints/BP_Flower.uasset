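; Flower actor that gradually grows in random steps after it spawns.
; BeginPlay starts a growth event that chains twelve identical stages, each passing a high-probability roll before a random delay of several seconds and a small uniform increase to the StaticMesh scale.
; A failed roll ends growth for good, so final sizes vary between flowers.
; Each step adds to the world scale but writes it as relative scale.
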(event `Grow_Up`
  (bind _staticmesh (`self.StaticMesh`))
  (bind _staticmesh_2 (`self.StaticMesh`))
  (bind _staticmesh_3 (`self.StaticMesh`))
  (bind _staticmesh_4 (`self.StaticMesh`))
  (bind _staticmesh_5 (`self.StaticMesh`))
  (bind _staticmesh_6 (`self.StaticMesh`))
  (bind _staticmesh_7 (`self.StaticMesh`))
  (bind _staticmesh_8 (`self.StaticMesh`))
  (bind _staticmesh_9 (`self.StaticMesh`))
  (bind _staticmesh_10 (`self.StaticMesh`))
  (bind _staticmesh_11 (`self.StaticMesh`))
  (bind _staticmesh_12 (`self.StaticMesh`))
  (if (`KismetMathLibrary.RandomBoolWithWeight` 0.9)
    (`KismetSystemLibrary.Delay` (`KismetMathLibrary.RandomFloatInRange` 5.0 15.0))
    (`SceneComponent.SetRelativeScale3D` _staticmesh_9 (+ (`SceneComponent.K2_GetComponentScale` _staticmesh_9) (0.1 0.1 0.1)))
    (if (`KismetMathLibrary.RandomBoolWithWeight` 0.9)
      (`KismetSystemLibrary.Delay` (`KismetMathLibrary.RandomFloatInRange` 5.0 15.0))
      (`SceneComponent.SetRelativeScale3D` _staticmesh_10 (+ (`SceneComponent.K2_GetComponentScale` _staticmesh_10) (0.1 0.1 0.1)))
      (if (`KismetMathLibrary.RandomBoolWithWeight` 0.9)
        (`KismetSystemLibrary.Delay` (`KismetMathLibrary.RandomFloatInRange` 5.0 15.0))
        (`SceneComponent.SetRelativeScale3D` _staticmesh_11 (+ (`SceneComponent.K2_GetComponentScale` _staticmesh_11) (0.1 0.1 0.1)))
        (if (`KismetMathLibrary.RandomBoolWithWeight` 0.9)
          (`KismetSystemLibrary.Delay` (`KismetMathLibrary.RandomFloatInRange` 5.0 15.0))
          (`SceneComponent.SetRelativeScale3D` _staticmesh_12 (+ (`SceneComponent.K2_GetComponentScale` _staticmesh_12) (0.1 0.1 0.1)))
          (if (`KismetMathLibrary.RandomBoolWithWeight` 0.9)
            (`KismetSystemLibrary.Delay` (`KismetMathLibrary.RandomFloatInRange` 5.0 15.0))
            (`SceneComponent.SetRelativeScale3D` _staticmesh_2 (+ (`SceneComponent.K2_GetComponentScale` _staticmesh_2) (0.1 0.1 0.1)))
            (if (`KismetMathLibrary.RandomBoolWithWeight` 0.9)
              (`KismetSystemLibrary.Delay` (`KismetMathLibrary.RandomFloatInRange` 5.0 15.0))
              (`SceneComponent.SetRelativeScale3D` _staticmesh_3 (+ (`SceneComponent.K2_GetComponentScale` _staticmesh_3) (0.1 0.1 0.1)))
              (if (`KismetMathLibrary.RandomBoolWithWeight` 0.9)
                (`KismetSystemLibrary.Delay` (`KismetMathLibrary.RandomFloatInRange` 5.0 15.0))
                (`SceneComponent.SetRelativeScale3D` _staticmesh_4 (+ (`SceneComponent.K2_GetComponentScale` _staticmesh_4) (0.1 0.1 0.1)))
                (if (`KismetMathLibrary.RandomBoolWithWeight` 0.9)
                  (`KismetSystemLibrary.Delay` (`KismetMathLibrary.RandomFloatInRange` 5.0 15.0))
                  (`SceneComponent.SetRelativeScale3D` _staticmesh_5 (+ (`SceneComponent.K2_GetComponentScale` _staticmesh_5) (0.1 0.1 0.1)))
                  (if (`KismetMathLibrary.RandomBoolWithWeight` 0.9)
                    (`KismetSystemLibrary.Delay` (`KismetMathLibrary.RandomFloatInRange` 5.0 15.0))
                    (`SceneComponent.SetRelativeScale3D` _staticmesh_6 (+ (`SceneComponent.K2_GetComponentScale` _staticmesh_6) (0.1 0.1 0.1)))
                    (if (`KismetMathLibrary.RandomBoolWithWeight` 0.9)
                      (`KismetSystemLibrary.Delay` (`KismetMathLibrary.RandomFloatInRange` 5.0 15.0))
                      (`SceneComponent.SetRelativeScale3D` _staticmesh_7 (+ (`SceneComponent.K2_GetComponentScale` _staticmesh_7) (0.1 0.1 0.1)))
                      (if (`KismetMathLibrary.RandomBoolWithWeight` 0.9)
                        (`KismetSystemLibrary.Delay` (`KismetMathLibrary.RandomFloatInRange` 5.0 15.0))
                        (`SceneComponent.SetRelativeScale3D` _staticmesh_8 (+ (`SceneComponent.K2_GetComponentScale` _staticmesh_8) (0.1 0.1 0.1)))
                        (if (`KismetMathLibrary.RandomBoolWithWeight` 0.9)
                          (`KismetSystemLibrary.Delay` (`KismetMathLibrary.RandomFloatInRange` 5.0 15.0))
                          (`SceneComponent.SetRelativeScale3D` _staticmesh (+ (`SceneComponent.K2_GetComponentScale` _staticmesh) (0.1 0.1 0.1))))))))))))))))

(event `self.ReceiveBeginPlay`
  (`self.Grow_Up`))

(fn `UserConstructionScript`)