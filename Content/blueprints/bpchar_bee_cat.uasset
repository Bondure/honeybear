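; Bee cat character that hops around and delivers honey to the cat summoner actor.
; A Delay on Tick launches it up and along world X every 10 to 20 seconds.
; When the player pawn enters its Sphere, it launches itself in a random upward direction.
; When its Box overlaps the summoner, it adds a hundredth of its HoneyValue to that actor's Honey and empties its own.
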(event `self.ReceiveBeginPlay`
  (`parent.ReceiveBeginPlay`))

(event `self.ReceiveActorBeginOverlap`
  (params (OtherActor :type "Actor Object Reference"))
  (`parent.ReceiveActorBeginOverlap` OtherActor))

(event `self.ReceiveTick`
  (params (DeltaSeconds :type "Float (single-precision)"))
  (`parent.ReceiveTick` DeltaSeconds)
  (`KismetSystemLibrary.Delay` (`KismetMathLibrary.RandomFloatInRange` 10.0 20.0))
  (`self.LaunchCharacter` (400.0 0.0 1200.0)))

(event `self.Sphere.OnComponentBeginOverlap`
  (params (OverlappedComponent :type "PrimitiveComponent Object Reference") (OtherActor :type "Actor Object Reference") (OtherComp :type "PrimitiveComponent Object Reference") (OtherBodyIndex :type Integer) (bFromSweep :type Boolean) (SweepResult :type "HitResult Structure (by ref)"))
  (if (== OtherActor (`GameplayStatics.GetPlayerPawn` 0))
    (`self.LaunchCharacter` (`KismetMathLibrary.MakeVector` (`KismetMathLibrary.RandomFloatInRange` -800.0 800.0) (`KismetMathLibrary.RandomFloatInRange` -800.0 800.0) (`KismetMathLibrary.RandomFloatInRange` 1000.0 1500.0)))))

(event `self.Box.OnComponentBeginOverlap`
  (params (OverlappedComponent :type "PrimitiveComponent Object Reference") (OtherActor :type "Actor Object Reference") (OtherComp :type "PrimitiveComponent Object Reference") (OtherBodyIndex :type Integer) (bFromSweep :type Boolean) (SweepResult :type "HitResult Structure (by ref)"))
  (if (== (`GameplayStatics.GetObjectClass` OtherActor) "/Game/blueprints/bpac_sumoner/bpactor_sumoner_cat.bpactor_sumoner_cat_C")
    (bind _asbpactor_sumoner_cat (cast `/Game/blueprints/bpac_sumoner/bpactor_sumoner_cat` OtherActor))
    (set `/Game/blueprints/bpac_sumoner/bpactor_sumoner.Honey` (+ (`/Game/blueprints/bpac_sumoner/bpactor_sumoner.Honey` _asbpactor_sumoner_cat) (/ (`self.HoneyValue`) 100.0)) _asbpactor_sumoner_cat)
    (set `self.HoneyValue` 0.0)))

(fn `UserConstructionScript`
  (`parent.UserConstructionScript`))