(event `self.ReceiveBeginPlay`)

(event `CreateZ`
  (bind _returnvalue (`self.GetTransform`))
  (`|SpawnActorFromClass` "/Game/blueprints/bpac_build.bpac_build_C" (`KismetMathLibrary.MakeTransform` (.location _returnvalue) (`KismetMathLibrary.MakeRotator` (.roll (.rotation _returnvalue)) (.pitch (.rotation _returnvalue)) (- (.yaw (.rotation _returnvalue)) 90.0)) (* (.scale _returnvalue) (1.2 1.2 1.2))) "Undefined" "MultiplyWithRoot" null null)
  (`KismetArrayLibrary.Array_Add` (`self.Builds`) self))

(event `CreateM`
  (bind _returnvalue (`self.GetTransform`))
  (`|SpawnActorFromClass` "/Game/Fantastic_Village_Pack/blueprints/buildings/BP_BLD_house_14.BP_BLD_house_14_C" (`KismetMathLibrary.MakeTransform` (.location _returnvalue) (`KismetMathLibrary.MakeRotator` (.roll (.rotation _returnvalue)) (.pitch (.rotation _returnvalue)) (- (.yaw (.rotation _returnvalue)) -90.0)) (.scale _returnvalue)) "Undefined" "MultiplyWithRoot" null null)
  (`KismetArrayLibrary.Array_Add` (`self.Builds`) self))

(fn `IsSelf`
  (returns (`IsSelf?` :type Boolean))
  (for (_array_element _array_index) (`self.Builds`)
    (if (== _array_element (`|GetArrayItem` (`self.Builds`) _array_index))
      (return true)))
  (return false))

(fn `UserConstructionScript`)