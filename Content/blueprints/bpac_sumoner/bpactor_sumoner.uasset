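; Summoner actor that, when flagged as a beehive, periodically spawns bees around itself.
; Tick accumulates time up to a randomly re-rolled interval, then spawns the configured bee class at a random reachable navigation point nearby.
; A bee counter on the first-person player character caps the population and increments with each spawn.
; After a short delay, each new bee receives a SpawnOptimize call.
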(event `self.ReceiveTick`
  (params (DeltaSeconds :type "Float (single-precision)"))
  (if (`self.ItIsBeehive?`)
    (bind _asbp_first_person_character (cast `/Game/FirstPerson/Blueprints/BP_FirstPersonCharacter` (`GameplayStatics.GetPlayerPawn` 0)))
    (if (not (> (`/Game/FirstPerson/Blueprints/BP_FirstPersonCharacter.int_bee_on_,map` _asbp_first_person_character) 3000))
      (bind _output_get (set `self.float_time` (+ (`self.float_time`) DeltaSeconds)))
      (if (> _output_get (`self.time_for_spawn`))
        (set `self.float_time` 0.0)
        (set `self.time_for_spawn` (`KismetMathLibrary.RandomIntegerInRange` 3 5))
        (bind _returnvalue (`|SpawnActorFromClass` (`self.class_of_bee`) (`KismetMathLibrary.MakeTransform` (`NavigationSystemV1.K2_GetRandomReachablePointInRadius` (`SceneComponent.K2_GetComponentLocation` (`self.DefaultSceneRoot`)) 200.0 null null)) "Undefined" "MultiplyWithRoot" null null))
        (bind _asbp_first_person_character_2 (cast `/Game/FirstPerson/Blueprints/BP_FirstPersonCharacter` (`GameplayStatics.GetPlayerPawn` 0)))
        (set `/Game/FirstPerson/Blueprints/BP_FirstPersonCharacter.int_bee_on_,map` (+ (`/Game/FirstPerson/Blueprints/BP_FirstPersonCharacter.int_bee_on_,map` _asbp_first_person_character_2) 1) _asbp_first_person_character_2)
        (`KismetSystemLibrary.Delay` 1.0)
        (`/Game/blueprints/bpchar_bee.SpawnOptimize` _returnvalue)))))

(fn `UserConstructionScript`)