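; This actor is an activity generator that keeps spawning Bpchild_dieingturtle actors at random spots around a central point.
; Tick accumulates a timer and, past a two-second threshold, counts Bp_mainaction actors against a population cap.
; Below the cap, it traces downward from a random point in a box and spawns at the hit location with random yaw.
; The timer resets only on spawning, and the trace result is used without a hit check.
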(event `self.ReceiveTick`
  (params (DeltaSeconds :type "Float (single-precision)"))
  (bind (_returnvalue_roll _returnvalue_pitch _returnvalue_yaw) (`KismetMathLibrary.BreakRotator` (`KismetMathLibrary.RandomRotator` false)))
  (bind (_returnvalue_x _returnvalue_y _returnvalue_z) (`KismetMathLibrary.BreakVector` (`KismetMathLibrary.RandomPointInBoundingBox` (`self.midl_of_point_spawm`) (3000.0 3000.0 10.0))))
  (bind _output_get (set `self.timer` (+ DeltaSeconds (`self.timer`))))
  (if (> _output_get 2.0)
    (bind _outactors (`GameplayStatics.GetAllActorsOfClass` "/Game/blueprints/activitis/avtions/bp_mainaction.bp_mainaction_C"))
    (if (< (`KismetArrayLibrary.Array_Length` _outactors) 31)
      (bind _outhit (`KismetSystemLibrary.LineTraceSingle` (`KismetMathLibrary.MakeVector` _returnvalue_x _returnvalue_y _returnvalue_z) (`KismetMathLibrary.MakeVector` _returnvalue_x _returnvalue_y -1000.0) "TraceTypeQuery1"))
      (`|SpawnActorFromClass` "/Game/blueprints/activitis/avtions/bpchild_dieingturtle.bpchild_dieingturtle_C" (`KismetMathLibrary.MakeTransform` (`.Location` (`GameplayStatics.BreakHitResult` _outhit)) (`KismetMathLibrary.MakeRotator` 0.0 0.0 _returnvalue_yaw)) "Undefined" "MultiplyWithRoot" null null)
      (set `self.timer` 0.0))))

(fn `UserConstructionScript`)