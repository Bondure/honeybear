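; Lab actor that consumes bees entering its box and changes its mesh material to match the bee's type.
; On overlap it ignores hits from components of the same class as the bee's optimization sphere, then uses a cast chain to pick a cat, ice, jungle, rock, lava or default material.
; DeltaMat applies CurrentMat at BeginPlay and after each pick, while CleanCurrentMat only resets the variable to the clean material.
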(event `CleanCurrentMat`
  (set `self.CurrentMat` "/Game/blueprints/widgets/2d_for_widgets/MatForLab/clean__2__Mat.clean__2__Mat"))

(event `DeltaMat`
  (`PrimitiveComponent.SetMaterial` (`self.StaticMesh`) 0 (`self.CurrentMat`)))

(event `self.ReceiveBeginPlay`
  (`self.DeltaMat`))

(event `self.Box.OnComponentBeginOverlap`
  (params (OverlappedComponent :type "PrimitiveComponent Object Reference") (OtherActor :type "Actor Object Reference") (OtherComp :type "PrimitiveComponent Object Reference") (OtherBodyIndex :type Integer) (bFromSweep :type Boolean) (SweepResult :type "HitResult Structure (by ref)"))
  (bind _asbpchar_bee (cast `/Game/blueprints/bpchar_bee` OtherActor))
  (if (not (== (`GameplayStatics.GetObjectClass` (`/Game/blueprints/bpchar_bee.SphereforOptimization` _asbpchar_bee)) (`GameplayStatics.GetObjectClass` OtherComp)))
    (cast `/Game/blueprints/bpchar_bee_cat` OtherActor
      (:`then`
        (set `self.CurrentMat` "/Game/blueprints/widgets/2d_for_widgets/MatForLab/кошачья__2__Mat.кошачья__2__Mat"))
      (:`CastFailed`
        (cast `/Game/blueprints/bpchar_bee_ice` OtherActor
          (:`then`
            (set `self.CurrentMat` "/Game/blueprints/widgets/2d_for_widgets/MatForLab/ледяная__2__Mat.ледяная__2__Mat"))
          (:`CastFailed`
            (cast `/Game/blueprints/bpchar_bee_jungke` OtherActor
              (:`then`
                (set `self.CurrentMat` "/Game/blueprints/widgets/2d_for_widgets/MatForLab/джунглевая__2__Mat.джунглевая__2__Mat"))
              (:`CastFailed`
                (cast `/Game/blueprints/bpchar_bee_rock` OtherActor
                  (:`then`
                    (set `self.CurrentMat` "/Game/blueprints/widgets/2d_for_widgets/MatForLab/горная__2__Mat.горная__2__Mat"))
                  (:`CastFailed`
                    (cast `/Game/blueprints/BPchar_lava_bee` OtherActor
                      (:`then`
                        (set `self.CurrentMat` "/Game/blueprints/widgets/2d_for_widgets/MatForLab/лавовая__2__Mat.лавовая__2__Mat"))
                      (:`CastFailed`
                        (set `self.CurrentMat` "/Game/blueprints/widgets/2d_for_widgets/MatForLab/обычная_Mat.обычная_Mat")))))))))))
    (`self.DeltaMat`)
    (`self.K2_DestroyActor` OtherActor)))

(fn `UserConstructionScript`)