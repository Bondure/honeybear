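; Global backend client, likely the GameInstance, that talks to the 2025.nti-gamedev.ru games REST API over HTTP with JSON.
; RegGame registers the team's game, signing headers with an MD5 of a fixed number plus a homemade UTC-based timestamp nonce from GetUnix.
; RegPlayer posts name, Money and HoneyPrice entries, GetRes fetches them back into variables, and CreateLogs posts comments.
; Player and log URLs use a UUID that this graph never sets.
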(event `Reg Game`
  (bind _jsonobjectwrapper (make `JsonObjectWrapper`))
  (bind _headers (`self.Headers`))
  (bind _unix (`self.GetUNIX`))
  (bind _output_get (set `self.T+U` (+ 604839 _unix)))
  (bind _returnvalue (`MD5Final.ComputeMD5Hash` (`KismetStringLibrary.Concat_StrStr` "604839" (`KismetStringLibrary.Conv_Int64ToString` _unix))))
  (`|SetJsonField` _jsonobjectwrapper "TeamName" (`self.Str`))
  (bind _outjsonstring (`JsonBlueprintFunctionLibrary.ToString` _jsonobjectwrapper))
  (`HttpBlueprintFunctionLibrary.AddHeader` _headers "Nonce" (`KismetStringLibrary.Conv_Int64ToString` _unix))
  (`HttpBlueprintFunctionLibrary.AddHeader` _headers "Talant-Id" "411452")
  (`HttpBlueprintFunctionLibrary.AddHeader` _headers "Signature" _returnvalue)
  (bind _returnvalue_2 (`HttpRequestProxyObject.CreateHttpRequestProxyObject` "https://2025.nti-gamedev.ru/api/games/" "POST" (`self.Headers`) (`KismetStringLibrary.Concat_StrStr` "" _outjsonstring)))
  (add `HttpRequestProxyObject.OnRequestComplete` _returnvalue_2 (delegate `ResponceGame`)))

(event `ResponceGame`
  (params (Response :type String) (bSuccessful :type Boolean) (OutHeader :type "HttpHeader Structure"))
  (`KismetSystemLibrary.PrintString` Response true true (struct :`G` 0.66 :`B` 1.0 :`A` 1.0) 1000.0)
  (`KismetSystemLibrary.PrintString` (`KismetStringLibrary.Concat_StrStr` "604839" (`KismetStringLibrary.Conv_Int64ToString` (stale `Reg Game` _unix))) true true (struct :`G` 0.66 :`B` 1.0 :`A` 1.0) 1000.0)
  (`KismetSystemLibrary.PrintString` (stale `Reg Game` _returnvalue) true true (struct :`G` 0.66 :`B` 1.0 :`A` 1.0) 1000.0))

(event `Reg Player`
  (bind _jsonobjectwrapper (make `JsonObjectWrapper`))
  (`|SetJsonField` _jsonobjectwrapper "Name" (`self.UserName`))
  (`|SetJsonField` _jsonobjectwrapper "Money" (`self.Money`))
  (for _index (range 6)
    (`|SetJsonField` _jsonobjectwrapper (`KismetStringLibrary.Concat_StrStr` "HoneyPrice" (`KismetStringLibrary.Conv_IntToString` _index)) (`|GetArrayItem` (`self.HoneyPrice`) _index)))
  (bind _outjsonstring (`|StructToJsonString` (make `RigVMFunction_StringConcat` (`self.UUID`) "\"/players/\"")))
  (bind _outjsonstring_2 (`JsonBlueprintFunctionLibrary.ToString` _jsonobjectwrapper))
  (`HttpRequestProxyObject.CreateHttpRequestProxyObject` (`KismetStringLibrary.Concat_StrStr` "https://2025.nti-gamedev.ru/api/games/" _outjsonstring) "POST" (`self.HeaderPlayer`) _outjsonstring_2))

(event `GetRes`
  (bind _outjsonstring (`|StructToJsonString` (make `RigVMFunction_StringConcat` (`KismetStringLibrary.Concat_StrStr` (`self.UUID`) "/players/") (`self.UserName`))))
  (bind _returnvalue (`HttpRequestProxyObject.CreateHttpRequestProxyObject` (`KismetStringLibrary.Concat_StrStr` "https://2025.nti-gamedev.ru/api/games/" _outjsonstring) "Get"))
  (add `HttpRequestProxyObject.OnRequestComplete` _returnvalue (delegate `ResultsRes`)))

(event `ResultsRes`
  (params (Response :type String) (bSuccessful :type Boolean) (OutHeader :type "HttpHeader Structure"))
  (bind _returnvalue (`KismetStringLibrary.Concat_StrStr` "HoneyPrice" (`KismetStringLibrary.Conv_IntToString` (`self.A`))))
  (set `self.A` 0)
  (bind _outjsonobject (`JsonBlueprintFunctionLibrary.FromString` Response))
  (bind _outvalue (`|GetJsonField` _outjsonobject "Money"))
  (set `self.Money` _outvalue)
  (bind _outvalue_2 (`|GetJsonField` _outjsonobject _returnvalue))
  (set `self.A` (+ (`self.A`) 1))
  (bind _outvalue_3 (`|GetJsonField` _outjsonobject _returnvalue))
  (set `self.A` (+ (`self.A`) 1))
  (bind _outvalue_4 (`|GetJsonField` _outjsonobject _returnvalue))
  (set `self.A` (+ (`self.A`) 1))
  (bind _outvalue_5 (`|GetJsonField` _outjsonobject _returnvalue))
  (set `self.A` (+ (`self.A`) 1))
  (bind _outvalue_6 (`|GetJsonField` _outjsonobject _returnvalue))
  (set `self.HoneyPrice` (`|MakeArray` _outvalue_2 _outvalue_3 _outvalue_4 _outvalue_5 _outvalue_6)))

(event `Create Logs`
  (bind _outjsonstring (`|StructToJsonString` (make `RigVMFunction_StringConcat` (`KismetStringLibrary.Concat_StrStr` (`self.UUID`) "/logs") (`self.UserName`))))
  (`HttpRequestProxyObject.CreateHttpRequestProxyObject` (`KismetStringLibrary.Concat_StrStr` "https://2025.nti-gamedev.ru/api/games/" _outjsonstring) "POST" (struct) (`KismetStringLibrary.Concat_StrStr` "{ \n   \"comment\":" (`self.Comment`) "}")))

(fn `GetUnix`
  (returns (Unix :type Integer64))
  (bind (_returnvalue_year _returnvalue_month _returnvalue_day _returnvalue_hour _returnvalue_minute _returnvalue_second) (`KismetMathLibrary.BreakDateTime` (`KismetMathLibrary.UtcNow`)))
  (return (+ 1012326827 (+ _returnvalue_second (`KismetMathLibrary.Abs_Int` (* _returnvalue_minute 60)) (`KismetMathLibrary.Abs_Int` (* _returnvalue_hour 3600)) (`KismetMathLibrary.Abs_Int` (* _returnvalue_day 86400)) (`KismetMathLibrary.Abs_Int` (* _returnvalue_month 2592000)) (`KismetMathLibrary.Abs_Int` (* _returnvalue_year 946080000))))))