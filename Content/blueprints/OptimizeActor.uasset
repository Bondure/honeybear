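; OptimizeActor is a proximity-triggered placeholder that defers spawning of an actor until the player comes near.
; When the capsule of BP_FirstPersonCharacter overlaps SphereforOptimization, the Spawn event creates an actor of class Char at CharTransform, ignoring collisions.
; The placeholder then destroys itself, so the spawn happens only once, and Tick does no work.
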(event `Spawn`
  (`|SpawnActorFromClass` (`self.Char`) (`self.CharTransform`) "AlwaysSpawn" "MultiplyWithRoot" null null)
  (`self.K2_DestroyActor`))

(event `self.SphereforOptimization.OnComponentBeginOverlap`
  (params (OverlappedComponent :type "PrimitiveComponent Object Reference") (OtherActor :type "Actor Object Reference") (OtherComp :type "PrimitiveComponent Object Reference") (OtherBodyIndex :type Integer) (bFromSweep :type Boolean) (SweepResult :type "HitResult Structure (by ref)"))
  (bind _asbp_first_person_character (cast `/Game/FirstPerson/Blueprints/BP_FirstPersonCharacter` OtherActor))
  (if (== OtherComp (`Character.CapsuleComponent` _asbp_first_person_character))
    (`self.Spawn`)))

(fn `UserConstructionScript`)