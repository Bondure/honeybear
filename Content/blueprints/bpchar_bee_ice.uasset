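; Ice bee character that hampers the player at close range and delivers honey to a frost summoner.
; Overlapping Sphere slows the player through CustomTimeDilation until exit, while Sphere1 sets a flag that lets a looping one-second timer call the player's FireX.
; Some_sad_box overlaps accept only the frost summoner class, then add scaled HoneyValue to its Honey (trying an ice beehive cast first) and zero the bee's load.
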(event `self.ReceiveBeginPlay`
  (`parent.ReceiveBeginPlay`)
  (`KismetSystemLibrary.K2_SetTimerDelegate` (delegate `What?`) 1.0 true))

(event `What?`
  (if (`self.?`)
    (bind _asbp_first_person_character (cast `/Game/FirstPerson/Blueprints/BP_FirstPersonCharacter` (`GameplayStatics.GetPlayerPawn` 0)))
    (`/Game/FirstPerson/Blueprints/BP_FirstPersonCharacter.FireX` _asbp_first_person_character)))

(event `self.ReceiveActorBeginOverlap`
  (params (OtherActor :type "Actor Object Reference"))
  (`parent.ReceiveActorBeginOverlap` OtherActor))

(event `self.ReceiveTick`
  (params (DeltaSeconds :type "Float (single-precision)"))
  (`parent.ReceiveTick` DeltaSeconds))

(event `self.Sphere1.OnComponentBeginOverlap`
  (params (OverlappedComponent :type "PrimitiveComponent Object Reference") (OtherActor :type "Actor Object Reference") (OtherComp :type "PrimitiveComponent Object Reference") (OtherBodyIndex :type Integer) (bFromSweep :type Boolean) (SweepResult :type "HitResult Structure (by ref)"))
  (if (== OtherActor (`GameplayStatics.GetPlayerPawn` 0))
    (set `self.?` true)))

(event `self.Sphere1.OnComponentEndOverlap`
  (params (OverlappedComponent :type "PrimitiveComponent Object Reference") (OtherActor :type "Actor Object Reference") (OtherComp :type "PrimitiveComponent Object Reference") (OtherBodyIndex :type Integer))
  (if (== OtherActor (`GameplayStatics.GetPlayerPawn` 0))
    (set `self.?` false)))

(event `self.Sphere.OnComponentBeginOverlap`
  (params (OverlappedComponent :type "PrimitiveComponent Object Reference") (OtherActor :type "Actor Object Reference") (OtherComp :type "PrimitiveComponent Object Reference") (OtherBodyIndex :type Integer) (bFromSweep :type Boolean) (SweepResult :type "HitResult Structure (by ref)"))
  (if (== OtherActor (`GameplayStatics.GetPlayerPawn` 0))
    (bind _asbp_first_person_character (cast `/Game/FirstPerson/Blueprints/BP_FirstPersonCharacter` OtherActor))
    (set `Actor.CustomTimeDilation` 0.125 _asbp_first_person_character)))

(event `self.Sphere.OnComponentEndOverlap`
  (params (OverlappedComponent :type "PrimitiveComponent Object Reference") (OtherActor :type "Actor Object Reference") (OtherComp :type "PrimitiveComponent Object Reference") (OtherBodyIndex :type Integer))
  (if (== OtherActor (`GameplayStatics.GetPlayerPawn` 0))
    (bind _asbp_first_person_character (cast `/Game/FirstPerson/Blueprints/BP_FirstPersonCharacter` OtherActor))
    (set `Actor.CustomTimeDilation` 1.0 _asbp_first_person_character)))

(event `self.some_sad_box.OnComponentBeginOverlap`
  (params (OverlappedComponent :type "PrimitiveComponent Object Reference") (OtherActor :type "Actor Object Reference") (OtherComp :type "PrimitiveComponent Object Reference") (OtherBodyIndex :type Integer) (bFromSweep :type Boolean) (SweepResult :type "HitResult Structure (by ref)"))
  (if (== (`GameplayStatics.GetObjectClass` OtherActor) "/Game/blueprints/bpac_sumoner/bpactor_sumoner_FROST.bpactor_sumoner_FROST_C")
    (bind _asbpactor_beehive_ice (cast `/Game/blueprints/bpac_sumoner/beehive/bpactor_beehive_ice` OtherActor)
      (:`then`
        (set `/Game/blueprints/bpac_sumoner/bpactor_sumoner.Honey` (+ (`/Game/blueprints/bpac_sumoner/bpactor_sumoner.Honey` _asbpactor_beehive_ice) (/ (`self.HoneyValue`) 100.0)) _asbpactor_beehive_ice)
        (set `self.HoneyValue` 0.0))
      (:`CastFailed`
        (bind _asbpactor_sumoner_frost (cast `/Game/blueprints/bpac_sumoner/bpactor_sumoner_FROST` OtherActor))
        (set `/Game/blueprints/bpac_sumoner/bpactor_sumoner.Honey` (+ (`/Game/blueprints/bpac_sumoner/bpactor_sumoner.Honey` _asbpactor_sumoner_frost) (/ (`self.HoneyValue`) 100.0)) _asbpactor_sumoner_frost)
        (set `self.HoneyValue` 0.0)))))

(fn `UserConstructionScript`
  (`parent.UserConstructionScript`))