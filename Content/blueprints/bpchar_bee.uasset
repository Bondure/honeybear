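; Bee character that flies and wanders by sending its AI controller to a random nearby navigable point every two seconds, without pathfinding.
; Suck events pause new wander orders and spin the bee via RotatingMovement until a timeout or end event resets rotation and resumes roaming.
; A separate event launches it with a given velocity in flying mode.
; Sine bobbing, physics toggle and population-cap destruction are disconnected leftovers.
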(event `set_ai_controller`
  (params (vellocity :type "Vector Structure"))
  (`CharacterMovementComponent.SetMovementMode` (`self.CharacterMovement`) "MOVE_Flying" 0)
  (`self.LaunchCharacter` vellocity))

(event `self.ReceiveBeginPlay`
  (`|ExecutionSequence`
    (:`then_0`
      (`KismetSystemLibrary.Delay` 0.3)
      (`CharacterMovementComponent.SetMovementMode` (`self.CharacterMovement`) "MOVE_Flying" 0)
      (bind _outactors (`GameplayStatics.GetAllActorsOfClass` "bpchar_bee_C")))
    (:`then_1`
      (`KismetSystemLibrary.K2_SetTimerDelegate` (delegate `Sin`) 1.0 true))))

(event `fuck_spawn`
  (set `self.spaw_form_wat` false))

(event `Sin`
  (set `self.time` (+ (`self.time`) 1.0)))

(event `self.ReceiveTick`
  (params (DeltaSeconds :type "Float (single-precision)"))
  (bind _timer (`self.timer`))
  (`|ExecutionSequence`
    (:`then_0`
      (set `self.timer` (+ _timer DeltaSeconds))
      (if (> _timer 2.0)
        (set `self.timer` 0.0)
        (if (not (`self.start_of_sucking`))
          (bind _randomlocation (`NavigationSystemV1.K2_GetRandomLocationInNavigableRadius` (`SceneComponent.K2_GetComponentLocation` (`self.CapsuleComponent`)) 1000.0 null null))
          (`AIController.MoveToLocation` (`AIBlueprintHelperLibrary.GetAIController` self) (`KismetMathLibrary.MakeVector` (.x _randomlocation) (.y _randomlocation) (.z _randomlocation)) -1.0 true false false true null true))))))

(event `suck_start`
  (set `RotatingMovementComponent.RotationRate` (struct :`Pitch` 340.0 :`Yaw` 340.0 :`Roll` 340.0) (`self.RotatingMovement`))
  (set `self.start_of_sucking` true)
  (`KismetSystemLibrary.Delay` 4.0)
  (set `self.start_of_sucking` false)
  (set `RotatingMovementComponent.RotationRate` (struct) (`self.RotatingMovement`))
  (bind _randomlocation (`NavigationSystemV1.K2_GetRandomLocationInNavigableRadius` (`SceneComponent.K2_GetComponentLocation` (`self.CapsuleComponent`)) 1000.0 null null))
  (`AIController.MoveToLocation` (`AIBlueprintHelperLibrary.GetAIController` self) _randomlocation -1.0 true true false true null true)
  (`SceneComponent.K2_SetWorldRotation` :`self` (`self.CapsuleComponent`) :`bSweep` true))

(event `suck_end`
  (set `RotatingMovementComponent.RotationRate` (struct) (`self.RotatingMovement`))
  (set `self.start_of_sucking` false)
  (bind _randomlocation (`NavigationSystemV1.K2_GetRandomLocationInNavigableRadius` (`SceneComponent.K2_GetComponentLocation` (`self.CapsuleComponent`)) 1000.0 null null))
  (`AIController.MoveToLocation` (`AIBlueprintHelperLibrary.GetAIController` self) _randomlocation -1.0 true true false true null true)
  (`SceneComponent.K2_SetWorldRotation` :`self` (`self.CapsuleComponent`) :`bSweep` true))

(fn `UserConstructionScript`)