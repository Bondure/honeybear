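; Valier actor that forms a resizable regular-polygon ring of Bpac_componentOfValier segments and tracks bees inside it.
; BeginPlay spawns five segments; mouse-wheel input changes the side count within limits, respawning segments and snapping them to the Landscape with vertical traces.
; Apothem trigonometry positions and rotates each segment and scales the detection Sphere to match.
; A looping timer refills BeeArray with overlapping Bpchar_bee actors whose VsosBull flag is set.
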(event `Different`
  (bind _returnvalue (`self.GetTransform`))
  (if (> (stale `MouseRoll` AxisValue) 0.0)
    (set `self.n` (+ (`self.n`) 1))
    (for _array_element (`self.ActorArray`) :!label _label
      (`self.K2_DestroyActor` _array_element))
    (`KismetArrayLibrary.Array_Clear` (`self.ActorArray`))
    (for _index (range 1 (+ (`self.n`) 1))
      (bind (_x _y) (`self.GetRelativeCoordinate` _index))
      (bind _angle (`self.GetRelativeTransform` _index))
      (bind _returnvalue_2 (`KismetMathLibrary.TransformLocation` _returnvalue (`KismetMathLibrary.MakeVector` _x _y)))
      (bind _returnvalue_3 (`|SpawnActorFromClass` "/Game/blueprints/bpac_componentOfValier.bpac_componentOfValier_C" (`KismetMathLibrary.MakeTransform` _returnvalue_2 (`KismetMathLibrary.TransformRotation` _returnvalue (`KismetMathLibrary.MakeRotator` 0.0 0.0 _angle))) "Undefined" "MultiplyWithRoot" null null))
      (`KismetArrayLibrary.Array_Add` (`self.ActorArray`) _returnvalue_3)
      (bind _outhits (`KismetSystemLibrary.LineTraceMulti` (- _returnvalue_2 (`KismetMathLibrary.MakeVector` 0.0 0.0 1000.0)) (+ _returnvalue_2 (`KismetMathLibrary.MakeVector` 0.0 0.0 1000.0)) "TraceTypeQuery1"))
      (for _array_element_2 _outhits
        (bind _returnvalue_4 (`GameplayStatics.GetActorOfClass` "/Script/Landscape.Landscape"))
        (if (== (`.HitActor` (`GameplayStatics.BreakHitResult` _array_element_2)) _returnvalue_4)
          (`self.K2_SetActorLocation` _returnvalue_3 (+ (`.ImpactPoint` (`GameplayStatics.BreakHitResult` _array_element_2)) (0.0 0.0 0.0)) false false))))
    (`self.SetCollisionScale`)
    (elif (< (stale `MouseRoll` AxisValue) 0.0)
      (set `self.n` (- (`self.n`) 1))
      (goto _label))))

(event `MouseRoll`
  (params (AxisValue :type "Float (double-precision)"))
  (bind _returnvalue (`KismetMathLibrary.Conv_DoubleToInt64` (+ (`self.n`) AxisValue)))
  (if (!= AxisValue 0.0)
    (if (> _returnvalue 50)
      (set `self.n` 50)
      (elif (< _returnvalue 5)
        (set `self.n` 4)
        (else
          (`self.Different`))))))

(event `self.ReceiveBeginPlay`
  (bind _returnvalue (`self.GetTransform`))
  (bind _returnvalue_2 (`self.GetTransform`))
  (bind _returnvalue_3 (`self.GetTransform`))
  (bind _returnvalue_4 (`self.GetTransform`))
  (bind _returnvalue_5 (`self.GetTransform`))
  (`|ExecutionSequence`
    (:`then_0`
      (bind _output_get (set `self.n` 5))
      (bind _r (`self.GetApofema` _output_get))
      (bind _output_get_2 (set `self.Start apofema` _r))
      (`self.SetCollisionScale`)
      (bind _output_get_3 (set `self.n` 5))
      (bind _r_2 (`self.GetApofema` _output_get_3))
      (bind (_x _y) (`self.GetRelativeCoordinate` 0))
      (bind _angle (`self.GetRelativeTransform` 0))
      (`KismetSystemLibrary.PrintString` (`KismetStringLibrary.Conv_DoubleToString` _angle) true true (struct :`G` 0.66 :`B` 1.0 :`A` 1.0) _angle)
      (bind _returnvalue_6 (`|SpawnActorFromClass` "/Game/blueprints/bpac_componentOfValier.bpac_componentOfValier_C" (`KismetMathLibrary.MakeTransform` (`KismetMathLibrary.TransformLocation` _returnvalue_2 (`KismetMathLibrary.MakeVector` _x _y)) (`KismetMathLibrary.TransformRotation` _returnvalue_2 (`KismetMathLibrary.MakeRotator` 0.0 0.0 _angle))) "AlwaysSpawn" "MultiplyWithRoot" null null))
      (`KismetArrayLibrary.Array_Add` (`self.ActorArray`) _returnvalue_6)
      (bind (_x_2 _y_2) (`self.GetRelativeCoordinate` 1))
      (bind _angle_2 (`self.GetRelativeTransform` 1))
      (`KismetSystemLibrary.PrintString` (`KismetStringLibrary.Conv_DoubleToString` _angle_2) true true (struct :`G` 0.66 :`B` 1.0 :`A` 1.0) _angle_2)
      (bind _returnvalue_7 (`|SpawnActorFromClass` "/Game/blueprints/bpac_componentOfValier.bpac_componentOfValier_C" (`KismetMathLibrary.MakeTransform` (`KismetMathLibrary.TransformLocation` _returnvalue_4 (`KismetMathLibrary.MakeVector` _x_2 _y_2)) (`KismetMathLibrary.TransformRotation` _returnvalue_4 (`KismetMathLibrary.MakeRotator` 0.0 0.0 _angle_2))) "AlwaysSpawn" "MultiplyWithRoot" null null))
      (`KismetArrayLibrary.Array_Add` (`self.ActorArray`) _returnvalue_7)
      (bind (_x_3 _y_3) (`self.GetRelativeCoordinate` 2))
      (bind _angle_3 (`self.GetRelativeTransform` 2))
      (`KismetSystemLibrary.PrintString` (`KismetStringLibrary.Conv_DoubleToString` _angle_3) true true (struct :`G` 0.66 :`B` 1.0 :`A` 1.0) _angle_3)
      (bind _returnvalue_8 (`|SpawnActorFromClass` "/Game/blueprints/bpac_componentOfValier.bpac_componentOfValier_C" (`KismetMathLibrary.MakeTransform` (`KismetMathLibrary.TransformLocation` _returnvalue_5 (`KismetMathLibrary.MakeVector` _x_3 _y_3)) (`KismetMathLibrary.TransformRotation` _returnvalue_5 (`KismetMathLibrary.MakeRotator` 0.0 0.0 _angle_3))) "AlwaysSpawn" "MultiplyWithRoot" null null))
      (`KismetArrayLibrary.Array_Add` (`self.ActorArray`) _returnvalue_8)
      (bind (_x_4 _y_4) (`self.GetRelativeCoordinate` 3))
      (bind _angle_4 (`self.GetRelativeTransform` 3))
      (`KismetSystemLibrary.PrintString` (`KismetStringLibrary.Conv_DoubleToString` _angle_4) true true (struct :`G` 0.66 :`B` 1.0 :`A` 1.0) _angle_4)
      (bind _returnvalue_9 (`|SpawnActorFromClass` "/Game/blueprints/bpac_componentOfValier.bpac_componentOfValier_C" (`KismetMathLibrary.MakeTransform` (`KismetMathLibrary.TransformLocation` _returnvalue (`KismetMathLibrary.MakeVector` _x_4 _y_4)) (`KismetMathLibrary.TransformRotation` _returnvalue (`KismetMathLibrary.MakeRotator` 0.0 0.0 _angle_4))) "AlwaysSpawn" "MultiplyWithRoot" null null))
      (`KismetArrayLibrary.Array_Add` (`self.ActorArray`) _returnvalue_9)
      (bind (_x_5 _y_5) (`self.GetRelativeCoordinate` 4))
      (bind _angle_5 (`self.GetRelativeTransform` 4))
      (`KismetSystemLibrary.PrintString` (`KismetStringLibrary.Conv_DoubleToString` _angle_5) true true (struct :`G` 0.66 :`B` 1.0 :`A` 1.0) _angle_5)
      (bind _returnvalue_10 (`|SpawnActorFromClass` "/Game/blueprints/bpac_componentOfValier.bpac_componentOfValier_C" (`KismetMathLibrary.MakeTransform` (`KismetMathLibrary.TransformLocation` _returnvalue_3 (`KismetMathLibrary.MakeVector` _x_5 _y_5)) (`KismetMathLibrary.TransformRotation` _returnvalue_3 (`KismetMathLibrary.MakeRotator` 0.0 0.0 _angle_5))) "AlwaysSpawn" "MultiplyWithRoot" null null))
      (`KismetArrayLibrary.Array_Add` (`self.ActorArray`) _returnvalue_10))
    (:`then_1`
      (`KismetSystemLibrary.K2_SetTimerDelegate` (delegate `CheckBeeInSphere`) 0.5 true))))

(event `SetCollisionScale`
  (bind _r (`self.GetApofema` (`self.n`)))
  (bind _returnvalue (* (/ _r (`self.Start apofema`)) 4.0))
  (`SceneComponent.SetRelativeScale3D` (`self.Sphere`) (`KismetMathLibrary.MakeVector` _returnvalue _returnvalue _returnvalue)))

(event `CheckActorsInSphere`
  (for _array_element (`PrimitiveComponent.GetOverlappingActors` (`self.Sphere`) null)
    (if (== (`GameplayStatics.GetObjectClass` _array_element) "/Game/blueprints/bpac_build.bpac_build_C")
      (set `self.ZInSphere` (`self.ZInSphere`))
      (break))))

(event `CheckBeeInSphere`
  (`KismetArrayLibrary.Array_Clear` (`self.BeeArray`))
  (for _array_element (`PrimitiveComponent.GetOverlappingActors` (`self.Sphere`) null)
    (if (or (== (`GameplayStatics.GetObjectClass` (`self.GetParentActor` _array_element)) "/Game/blueprints/bpchar_bee.bpchar_bee_C") (== (`GameplayStatics.GetObjectClass` _array_element) "/Game/blueprints/bpchar_bee.bpchar_bee_C"))
      (bind _asbpchar_bee (cast `/Game/blueprints/bpchar_bee` _array_element))
      (if (`/Game/blueprints/bpchar_bee.VsosBull?` _asbpchar_bee)
        (`KismetArrayLibrary.Array_Add` (`self.BeeArray`) _asbpchar_bee)))))

(fn `GetApofema`
  (params (n :type Integer))
  (returns (r :type "Float (double-precision)"))
  (return (/ (`self.a`) (* 2.0 (`KismetMathLibrary.Tan` (/ (`self.Pi`) n))))))

(fn `GetRelativeCoordinate`
  (params (i :type Integer))
  (returns (x :type "Float (double-precision)") (y :type "Float (double-precision)"))
  (return (* (/ (`self.a`) (* 2.0 (`KismetMathLibrary.Tan` (/ (`self.Pi`) (`self.n`))))) (`KismetMathLibrary.Cos` (/ (* (+ (* 2 i) 1) 3.141593) (`self.n`)))) (* (/ (`self.a`) (* 2.0 (`KismetMathLibrary.Tan` (/ (`self.Pi`) (`self.n`))))) (`KismetMathLibrary.Sin` (/ (* (+ (* 2.0 i) 1.0) 3.141593) (`self.n`))))))

(fn `GetRelativeTransform`
  (params (i :type Integer))
  (returns (angle :type "Float (double-precision)"))
  (return (`KismetMathLibrary.RadiansToDegrees` (+ (/ (`self.Pi`) 2.0) (/ (* 2.0 (`self.Pi`) (+ i 0.5)) (`self.n`))))))

(fn `UserConstructionScript`)