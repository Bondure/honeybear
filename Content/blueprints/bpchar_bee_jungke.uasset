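; Bee character that darts around by repeatedly launching itself in random horizontal directions, with a Niagara effect shown during each burst.
; BeginPlay hides the effect and, after a random delay, fires the first launch, then hands off to the Sprint event.
; Sprint repeats the same wait, launch and brief effect flash, calling itself again to loop indefinitely.
; Tick and overlap events only call their parents.
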(event `self.ReceiveBeginPlay`
  (`parent.ReceiveBeginPlay`)
  (`SceneComponent.SetVisibility` (`self.Niagara`) false false)
  (`KismetSystemLibrary.Delay` (`KismetMathLibrary.RandomFloatInRange` 0.0 2.0))
  (`SceneComponent.SetVisibility` (`self.Niagara`) true false)
  (`self.LaunchCharacter` (`KismetMathLibrary.MakeVector` (`KismetMathLibrary.RandomFloatInRange` -20000.0 20000.0) (`KismetMathLibrary.RandomFloatInRange` -20000.0 20000.0)))
  (`KismetSystemLibrary.Delay` 0.33)
  (`SceneComponent.SetVisibility` (`self.Niagara`) false false)
  (`self.Sprint`))

(event `self.ReceiveActorBeginOverlap`
  (params (OtherActor :type "Actor Object Reference"))
  (`parent.ReceiveActorBeginOverlap` OtherActor))

(event `self.ReceiveTick`
  (params (DeltaSeconds :type "Float (single-precision)"))
  (`parent.ReceiveTick` DeltaSeconds))

(event `Sprint`
  (`KismetSystemLibrary.Delay` (`KismetMathLibrary.RandomFloatInRange` 0.0 2.0))
  (`SceneComponent.SetVisibility` (`self.Niagara`) true false)
  (`self.LaunchCharacter` (`KismetMathLibrary.MakeVector` (`KismetMathLibrary.RandomFloatInRange` -20000.0 20000.0) (`KismetMathLibrary.RandomFloatInRange` -20000.0 20000.0)))
  (`KismetSystemLibrary.Delay` 0.33)
  (`SceneComponent.SetVisibility` (`self.Niagara`) false false)
  (`self.Sprint`))

(fn `UserConstructionScript`
  (`parent.UserConstructionScript`))