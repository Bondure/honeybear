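; BP_GrowUpFlower is a trigger actor that applies a one-time growth buff to BP_Flower actors.
; When an actor begins overlapping its Capsule, it checks for the exact BP_Flower class and casts to it.
; If the flower's BuffActive flag is unset, it calls GrowUp on the flower and then sets the flag, so an already buffed flower is skipped.
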(event `self.Capsule.OnComponentBeginOverlap`
  (params (OverlappedComponent :type "PrimitiveComponent Object Reference") (OtherActor :type "Actor Object Reference") (OtherComp :type "PrimitiveComponent Object Reference") (OtherBodyIndex :type Integer) (bFromSweep :type Boolean) (SweepResult :type "HitResult Structure (by ref)"))
  (if (== (`GameplayStatics.GetObjectClass` OtherActor) "/Game/blueprints/Flowers/BP_Flower.BP_Flower_C")
    (bind _asbp_flower (cast `/Game/blueprints/Flowers/BP_Flower` OtherActor))
    (if (not (`/Game/blueprints/Flowers/BP_Flower.BuffActive` _asbp_flower))
      (`self.Grow_Up` _asbp_flower)
      (set `/Game/blueprints/Flowers/BP_Flower.BuffActive` true _asbp_flower))))

(fn `UserConstructionScript`
  (`parent.UserConstructionScript`))