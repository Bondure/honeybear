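; BP_WoodFlower is a flower actor that strengthens and repairs traps and buildings within its capsule.
; On begin overlap, trap, build or house actors gain a permanent HP and MaxHP bonus and start a looping timer.
; Each timer tick gathers those classes world-wide, removes non-overlapping actors mid-loop, then adds a little HP where MaxHP allows.
; The heal chain also handles beehives, but the gather step never collects them.
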(event `self.Capsule.OnComponentBeginOverlap`
  (params (OverlappedComponent :type "PrimitiveComponent Object Reference") (OtherActor :type "Actor Object Reference") (OtherComp :type "PrimitiveComponent Object Reference") (OtherBodyIndex :type Integer) (bFromSweep :type Boolean) (SweepResult :type "HitResult Structure (by ref)"))
  (`|ExecutionSequence`
    (:`then_0`
      (bind _asbp_trap (cast `/Game/blueprints/BP_Trap` OtherActor))
      (set `/Game/blueprints/BP_Trap.HP` (+ (`/Game/blueprints/BP_Trap.HP` _asbp_trap) 50.0) _asbp_trap)
      (set `/Game/blueprints/BP_Trap.MaxHP` (+ (`/Game/blueprints/BP_Trap.MaxHP` _asbp_trap) 50.0) _asbp_trap))
    (:`then_1`
      (bind _asbpac_build (cast `/Game/blueprints/bpac_build` OtherActor))
      (set `/Game/blueprints/bpac_build.HP` (+ (`/Game/blueprints/bpac_build.HP` _asbpac_build) 50.0) _asbpac_build)
      (set `/Game/blueprints/bpac_build.MaxHP` (+ (`/Game/blueprints/bpac_build.MaxHP` _asbpac_build) 50.0) _asbpac_build))
    (:`then_2`
      (bind _asbuild (cast `/Game/blueprints/Build` OtherActor))
      (set `/Game/blueprints/Build.HP` (+ (`/Game/blueprints/Build.HP` _asbuild) 50.0) _asbuild)
      (set `/Game/blueprints/Build.MaxHP` (+ (`/Game/blueprints/Build.MaxHP` _asbuild) 50.0) _asbuild))
    (:`then_3`
      (bind _asbp_bld_house_14 (cast `/Game/Fantastic_Village_Pack/blueprints/buildings/BP_BLD_house_14` OtherActor))
      (set `/Game/Fantastic_Village_Pack/blueprints/buildings/BP_BLD_house_14.HP` (+ (`/Game/Fantastic_Village_Pack/blueprints/buildings/BP_BLD_house_14.HP` _asbp_bld_house_14) 50.0) _asbp_bld_house_14)
      (set `/Game/Fantastic_Village_Pack/blueprints/buildings/BP_BLD_house_14.MaxHP` (+ (`/Game/Fantastic_Village_Pack/blueprints/buildings/BP_BLD_house_14.MaxHP` _asbp_bld_house_14) 50.0) _asbp_bld_house_14)))
  (`KismetSystemLibrary.K2_SetTimerDelegate` (delegate `Tick`) 3.0 true))

(event `Tick`
  (`KismetArrayLibrary.Array_Clear` (`self.ActorsArray`))
  (bind _outactors (`GameplayStatics.GetAllActorsOfClass` "/Game/blueprints/BP_Trap.BP_Trap_C"))
  (bind _outactors_2 (`GameplayStatics.GetAllActorsOfClass` "/Game/blueprints/bpac_build.bpac_build_C"))
  (bind _outactors_3 (`GameplayStatics.GetAllActorsOfClass` "/Game/blueprints/Build.Build_C"))
  (bind _outactors_4 (`GameplayStatics.GetAllActorsOfClass` "/Game/Fantastic_Village_Pack/blueprints/buildings/BP_BLD_house_14.BP_BLD_house_14_C"))
  (for _array_element _outactors
    (`KismetArrayLibrary.Array_Add` (`self.ActorsArray`) _array_element))
  (for _array_element_2 _outactors_2
    (`KismetArrayLibrary.Array_Add` (`self.ActorsArray`) _array_element_2))
  (for _array_element_3 _outactors_3
    (`KismetArrayLibrary.Array_Add` (`self.ActorsArray`) _array_element_3))
  (for _array_element_4 _outactors_4
    (`KismetArrayLibrary.Array_Add` (`self.ActorsArray`) _array_element_4))
  (for _array_element_5 (`self.ActorsArray`)
    (if (not (`KismetArrayLibrary.Array_Contains` (`PrimitiveComponent.GetOverlappingActors` (`self.Capsule`) null) _array_element_5))
      (`KismetArrayLibrary.Array_RemoveItem` (`self.ActorsArray`) _array_element_5)))
  (for _array_element_6 (`self.ActorsArray`)
    (bind _asbp_trap (cast `/Game/blueprints/BP_Trap` _array_element_6)
      (:`then`
        (bind _returnvalue (+ (`/Game/blueprints/BP_Trap.HP` _asbp_trap) 3.0))
        (if (>= (`/Game/blueprints/BP_Trap.MaxHP` _asbp_trap) _returnvalue)
          (set `/Game/blueprints/BP_Trap.HP` _returnvalue _asbp_trap)))
      (:`CastFailed`
        (bind _asbpac_build (cast `/Game/blueprints/bpac_build` _array_element_6)
          (:`then`
            (bind _returnvalue_2 (+ (`/Game/blueprints/bpac_build.HP` _asbpac_build) 3.0))
            (if (>= (`/Game/blueprints/bpac_build.MaxHP` _asbpac_build) _returnvalue_2)
              (set `/Game/blueprints/bpac_build.HP` _returnvalue_2 _asbpac_build)))
          (:`CastFailed`
            (bind _asbuild (cast `/Game/blueprints/Build` _array_element_6)
              (:`then`
                (bind _returnvalue_3 (+ (`/Game/blueprints/Build.HP` _asbuild) 3.0))
                (if (>= (`/Game/blueprints/Build.MaxHP` _asbuild) _returnvalue_3)
                  (set `/Game/blueprints/Build.HP` _returnvalue_3 _asbuild)))
              (:`CastFailed`
                (bind _asbp_bld_house_14 (cast `/Game/Fantastic_Village_Pack/blueprints/buildings/BP_BLD_house_14` _array_element_6)
                  (:`then`
                    (bind _returnvalue_4 (+ (`/Game/Fantastic_Village_Pack/blueprints/buildings/BP_BLD_house_14.HP` _asbp_bld_house_14) 3.0))
                    (if (>= (`/Game/Fantastic_Village_Pack/blueprints/buildings/BP_BLD_house_14.MaxHP` _asbp_bld_house_14) _returnvalue_4)
                      (set `/Game/Fantastic_Village_Pack/blueprints/buildings/BP_BLD_house_14.HP` _returnvalue_4 _asbp_bld_house_14)))
                  (:`CastFailed`
                    (bind _asbpactor_beehive (cast `/Game/blueprints/bpac_sumoner/beehive/bpactor_beehive` _array_element_6))
                    (bind _returnvalue_5 (+ (`/Game/blueprints/bpac_sumoner/beehive/bpactor_beehive.HP` _asbpactor_beehive) 3.0))
                    (if (>= (`/Game/blueprints/bpac_sumoner/beehive/bpactor_beehive.MaxHP` _asbpactor_beehive) _returnvalue_5)
                      (set `/Game/blueprints/bpac_sumoner/beehive/bpactor_beehive.HP` _returnvalue_5 _asbpactor_beehive))))))))))))

(fn `UserConstructionScript`
  (`parent.UserConstructionScript`))