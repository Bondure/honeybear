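; BP_NoEnemyFlower is a flower that triggers "no enemy" calls on mobs that touch it.
; Its capsule's begin-overlap checks that the other actor's class is exactly Main_mob_logic, casts it, then calls NoenemyBee and NoenemyBuild on it.
; The effect of those calls lives in the mob; the flower has no other active logic.
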(event `self.Capsule.OnComponentBeginOverlap`
  (params (OverlappedComponent :type "PrimitiveComponent Object Reference") (OtherActor :type "Actor Object Reference") (OtherComp :type "PrimitiveComponent Object Reference") (OtherBodyIndex :type Integer) (bFromSweep :type Boolean) (SweepResult :type "HitResult Structure (by ref)"))
  (if (== (`GameplayStatics.GetObjectClass` OtherActor) "/Game/blueprints/mobs/main_mob_logic.main_mob_logic_C")
    (bind _asmain_mob_logic (cast `/Game/blueprints/mobs/main_mob_logic` OtherActor))
    (`/Game/blueprints/mobs/main_mob_logic.NoenemyBee` _asmain_mob_logic)
    (`/Game/blueprints/mobs/main_mob_logic.NoenemyBuild` _asmain_mob_logic)))

(fn `UserConstructionScript`
  (`parent.UserConstructionScript`))