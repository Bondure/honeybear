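; BP_PowerUpFlower is a flower that temporarily powers up the bee character while it overlaps the flower's capsule.
; On begin overlap, it checks for the bee class, raises the bee's MaxHoney and clears HeavyBool.
; End overlap is meant to lower MaxHoney and set HeavyBool, but its class comparison shows no connected input.
; BeginPlay and Tick are disabled stubs, so all logic lives in the overlap events.
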(event `self.Capsule.OnComponentBeginOverlap`
  (params (OverlappedComponent :type "PrimitiveComponent Object Reference") (OtherActor :type "Actor Object Reference") (OtherComp :type "PrimitiveComponent Object Reference") (OtherBodyIndex :type Integer) (bFromSweep :type Boolean) (SweepResult :type "HitResult Structure (by ref)"))
  (if (== (`GameplayStatics.GetObjectClass` OtherActor) "/Game/blueprints/bpchar_bee.bpchar_bee_C")
    (bind _asbpchar_bee (cast `/Game/blueprints/bpchar_bee` OtherActor))
    (set `/Game/blueprints/bpchar_bee.MaxHoney` 200.0 _asbpchar_bee)
    (set `/Game/blueprints/bpchar_bee.HeavyBool?` false _asbpchar_bee)))

(event `self.Capsule.OnComponentEndOverlap`
  (params (OverlappedComponent :type "PrimitiveComponent Object Reference") (OtherActor :type "Actor Object Reference") (OtherComp :type "PrimitiveComponent Object Reference") (OtherBodyIndex :type Integer))
  (if (== null "/Game/blueprints/bpchar_bee.bpchar_bee_C")
    (bind _asbpchar_bee (cast `/Game/blueprints/bpchar_bee` OtherActor))
    (set `/Game/blueprints/bpchar_bee.MaxHoney` 100.0 _asbpchar_bee)
    (set `/Game/blueprints/bpchar_bee.HeavyBool?` true _asbpchar_bee)))

(fn `UserConstructionScript`
  (`parent.UserConstructionScript`))