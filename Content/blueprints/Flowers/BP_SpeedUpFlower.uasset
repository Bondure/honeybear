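; Speed-up flower that boosts bees and other flowers while they are inside its capsule.
; On overlap begin it scales a BP_Flower's Factor down or doubles a bee's HoneySpeed, and on overlap end it applies the inverse.
; Targets are matched by exact class before casting, so child classes are not affected.
; An unconnected copy of the begin-overlap logic never runs.
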(event `self.Capsule.OnComponentBeginOverlap`
  (params (OverlappedComponent :type "PrimitiveComponent Object Reference") (OtherActor :type "Actor Object Reference") (OtherComp :type "PrimitiveComponent Object Reference") (OtherBodyIndex :type Integer) (bFromSweep :type Boolean) (SweepResult :type "HitResult Structure (by ref)"))
  (bind _returnvalue (`GameplayStatics.GetObjectClass` OtherActor))
  (if (== _returnvalue "/Game/blueprints/Flowers/BP_Flower.BP_Flower_C")
    (bind _asbp_flower (cast `/Game/blueprints/Flowers/BP_Flower` OtherActor))
    (set `/Game/blueprints/Flowers/BP_Flower.Factor` (* (`/Game/blueprints/Flowers/BP_Flower.Factor` _asbp_flower) 0.75) _asbp_flower)
    (elif (== _returnvalue "/Game/blueprints/bpchar_bee.bpchar_bee_C")
      (bind _asbpchar_bee (cast `/Game/blueprints/bpchar_bee` OtherActor))
      (set `/Game/blueprints/bpchar_bee.HoneySpeed` (* (`/Game/blueprints/bpchar_bee.HoneySpeed` _asbpchar_bee) 2.0) _asbpchar_bee))))

(event `self.Capsule.OnComponentEndOverlap`
  (params (OverlappedComponent :type "PrimitiveComponent Object Reference") (OtherActor :type "Actor Object Reference") (OtherComp :type "PrimitiveComponent Object Reference") (OtherBodyIndex :type Integer))
  (bind _returnvalue (`GameplayStatics.GetObjectClass` OtherActor))
  (if (== _returnvalue "/Game/blueprints/Flowers/BP_Flower.BP_Flower_C")
    (bind _asbp_flower (cast `/Game/blueprints/Flowers/BP_Flower` OtherActor))
    (set `/Game/blueprints/Flowers/BP_Flower.Factor` (/ (`/Game/blueprints/Flowers/BP_Flower.Factor` _asbp_flower) 0.75) _asbp_flower)
    (elif (== _returnvalue "/Game/blueprints/bpchar_bee.bpchar_bee_C")
      (bind _asbpchar_bee (cast `/Game/blueprints/bpchar_bee` OtherActor))
      (set `/Game/blueprints/bpchar_bee.HoneySpeed` (/ (`/Game/blueprints/bpchar_bee.HoneySpeed` _asbpchar_bee) 2.0) _asbpchar_bee))))

(fn `UserConstructionScript`
  (`parent.UserConstructionScript`))