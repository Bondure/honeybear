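; BP_Flower_Ice is an ice flower that gives honey to bees overlapping its capsule.
; An exact class check grants ice bees a boosted yield, while basic bees get a reduced yield or are randomly destroyed; other classes are ignored.
; Surviving bees receive honey after a delay set by their HoneySpeed, with no recheck of overlap, then run CheckOnMaxHoney.
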(event `self.Capsule.OnComponentBeginOverlap`
  (params (OverlappedComponent :type "PrimitiveComponent Object Reference") (OtherActor :type "Actor Object Reference") (OtherComp :type "PrimitiveComponent Object Reference") (OtherBodyIndex :type Integer) (bFromSweep :type Boolean) (SweepResult :type "HitResult Structure (by ref)"))
  (bind _returnvalue (`GameplayStatics.GetObjectClass` OtherActor))
  (if (== _returnvalue "/Game/blueprints/bpchar_bee_ice.bpchar_bee_ice_C")
    (set `self.Factor` 2.0)
    (bind _asbpchar_bee (cast `/Game/blueprints/bpchar_bee` OtherActor :!label _label))
    (`KismetSystemLibrary.Delay` (`/Game/blueprints/bpchar_bee.HoneySpeed` _asbpchar_bee))
    (set `/Game/blueprints/bpchar_bee.HoneyValue` (+ (`/Game/blueprints/bpchar_bee.HoneyValue` _asbpchar_bee) (* (`self.Factor`) 15.0)) _asbpchar_bee)
    (`KismetSystemLibrary.PrintString` "Hello")
    (`/Game/blueprints/bpchar_bee.CheckOnMaxHoney` _asbpchar_bee)
    (elif (== _returnvalue "/Game/blueprints/bpchar_bee.bpchar_bee_C")
      (set `self.Factor` 0.5)
      (if (`KismetMathLibrary.RandomBoolWithWeight` 0.25)
        (`self.K2_DestroyActor` OtherActor)
        (else
          (goto _label))))))

(fn `UserConstructionScript`
  (`parent.UserConstructionScript`))