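; Bee enclosure building that accumulates honey from the bees inside its box and has a movable fence door.
; Tick runs a one-minute timer that adds honey to a per-class map for each overlapping bee below a cap, doubled when a jungle bee is present.
; Text components show five bee types' totals every frame.
; Open and close events nudge the fence along the camera's forward vector, limited by a step counter.
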(event `self.ReceiveTick`
  (params (DeltaSeconds :type "Float (single-precision)"))
  (bind _quanity_honey (`self.quanity_honey`))
  (`|ExecutionSequence`
    (:`then_0`
      ;[1 1 1] накопление меда пчелами
      (bind _output_get (set `self.float_time` (+ (`self.float_time`) DeltaSeconds)))
      (if (> _output_get 60.0)
        (set `self.float_time` 0.0)
        (for _array_element (`PrimitiveComponent.GetOverlappingActors` (`self.Box`) "/Game/blueprints/bpchar_bee.bpchar_bee_C")
          (bind _asbpchar_bee (cast `/Game/blueprints/bpchar_bee` _array_element))
          (bind _value (`BlueprintMapLibrary.Map_Find` _quanity_honey (`GameplayStatics.GetObjectClass` _asbpchar_bee)))
          (if (< _value 30)
            (if (> (`KismetArrayLibrary.Array_Length` (`PrimitiveComponent.GetOverlappingActors` (`self.Box`) "/Game/blueprints/bpchar_bee_jungke.bpchar_bee_jungke_C")) 0)
              (bind _returnvalue (`GameplayStatics.GetObjectClass` _asbpchar_bee))
              (`BlueprintMapLibrary.Map_Add` _quanity_honey _returnvalue (+ _value 2))
              (else
                (`BlueprintMapLibrary.Map_Add` _quanity_honey _returnvalue (+ _value 1))))))))
    (:`then_1`
      (`TextRenderComponent.K2_SetText` (`self.normal`) (`KismetTextLibrary.Conv_IntToText` (`BlueprintMapLibrary.Map_Find` (`self.quanity_honey`) "/Game/blueprints/bpchar_bee.bpchar_bee_C")))
      (`TextRenderComponent.K2_SetText` (`self.lava`) (`KismetTextLibrary.Conv_IntToText` (`BlueprintMapLibrary.Map_Find` (`self.quanity_honey`) "/Game/blueprints/BPchar_lava_bee.BPchar_lava_bee_C")))
      (`TextRenderComponent.K2_SetText` (`self.rock`) (`KismetTextLibrary.Conv_IntToText` (`BlueprintMapLibrary.Map_Find` (`self.quanity_honey`) "/Game/blueprints/bpchar_bee_rock.bpchar_bee_rock_C")))
      (`TextRenderComponent.K2_SetText` (`self.ice`) (`KismetTextLibrary.Conv_IntToText` (`BlueprintMapLibrary.Map_Find` (`self.quanity_honey`) "/Game/blueprints/bpchar_bee_ice.bpchar_bee_ice_C")))
      (`TextRenderComponent.K2_SetText` (`self.cat`) (`KismetTextLibrary.Conv_IntToText` (`BlueprintMapLibrary.Map_Find` (`self.quanity_honey`) "/Game/blueprints/bpchar_bee_cat.bpchar_bee_cat_C"))))
    (:`then_2`
      (`KismetArrayLibrary.Array_Append` (`PrimitiveComponent.GetOverlappingActors` (`self.Box`) "/Game/blueprints/bpchar_bee.bpchar_bee_C") (`self.quanity_of_bee_types`)))))

(event `self.ReceiveBeginPlay`
  ;[1 1 1] накопление меда пчелами
  (set `self.vec_start_door_cord` (0.0 0.0 0.0)))

(event `close_door`
  (bind _sm_prop_fence_v01_02 (`self.SM_PROP_fence_v01_02`))
  (if (< (`self.int`) 0)
    (set `self.int` (+ (`self.int`) 2))
    (`SceneComponent.K2_SetWorldLocation` _sm_prop_fence_v01_02 (+ (`SceneComponent.K2_GetComponentLocation` _sm_prop_fence_v01_02) (* (`SceneComponent.GetForwardVector` (`self.Camera`)) (-2.0 -2.0 -2.0))) false false)))

(event `OPEN_DOOR`
  (bind _sm_prop_fence_v01_02 (`self.SM_PROP_fence_v01_02`))
  (bind _returnvalue (+ (`self.int`) -2))
  (if (> _returnvalue -170)
    (set `self.int` _returnvalue)
    (`SceneComponent.K2_SetWorldLocation` _sm_prop_fence_v01_02 (+ (`SceneComponent.K2_GetComponentLocation` _sm_prop_fence_v01_02) (* (`SceneComponent.GetForwardVector` (`self.Camera`)) (2.0 2.0 2.0))) false false)))

(fn `UserConstructionScript`)