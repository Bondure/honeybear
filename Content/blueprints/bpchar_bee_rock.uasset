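; Bee rock actor that reacts to the player and serves as a one-time honey source for the summoner mount.
; When the player enters its sphere, it shows a Niagara effect, calls Mud on the first-person character after a short delay, then hides the effect.
; When a summoner mount enters its box, it adds HoneyValue, scaled down by a hundred, to the mount's Honey and zeroes its own value.
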(event `self.ReceiveBeginPlay`
  (`parent.ReceiveBeginPlay`)
  (`SceneComponent.SetVisibility` (`self.Niagara`) false false))

(event `self.ReceiveActorBeginOverlap`
  (params (OtherActor :type "Actor Object Reference"))
  (`parent.ReceiveActorBeginOverlap` OtherActor))

(event `self.ReceiveTick`
  (params (DeltaSeconds :type "Float (single-precision)"))
  (`parent.ReceiveTick` DeltaSeconds))

(event `self.Sphere.OnComponentBeginOverlap`
  (params (OverlappedComponent :type "PrimitiveComponent Object Reference") (OtherActor :type "Actor Object Reference") (OtherComp :type "PrimitiveComponent Object Reference") (OtherBodyIndex :type Integer) (bFromSweep :type Boolean) (SweepResult :type "HitResult Structure (by ref)"))
  (if (== OtherActor (`GameplayStatics.GetPlayerPawn` 0))
    (`SceneComponent.SetVisibility` (`self.Niagara`) true false)
    (`KismetSystemLibrary.Delay` 0.4)
    (bind _asbp_first_person_character (cast `/Game/FirstPerson/Blueprints/BP_FirstPersonCharacter` OtherActor))
    (`/Game/FirstPerson/Blueprints/BP_FirstPersonCharacter.Mud` _asbp_first_person_character)
    (`KismetSystemLibrary.Delay` 1.5)
    (`SceneComponent.SetVisibility` (`self.Niagara`) false false)))

(event `self.Box.OnComponentBeginOverlap`
  (params (OverlappedComponent :type "PrimitiveComponent Object Reference") (OtherActor :type "Actor Object Reference") (OtherComp :type "PrimitiveComponent Object Reference") (OtherBodyIndex :type Integer) (bFromSweep :type Boolean) (SweepResult :type "HitResult Structure (by ref)"))
  (if (== (`GameplayStatics.GetObjectClass` OtherActor) "/Game/blueprints/bpac_sumoner/bpactor_sumoner_MOUNT.bpactor_sumoner_MOUNT_C")
    (bind _asbpactor_sumoner_mount (cast `/Game/blueprints/bpac_sumoner/bpactor_sumoner_MOUNT` OtherActor))
    (set `/Game/blueprints/bpac_sumoner/bpactor_sumoner.Honey` (+ (`/Game/blueprints/bpac_sumoner/bpactor_sumoner.Honey` _asbpactor_sumoner_mount) (/ (`self.HoneyValue`) 100.0)) _asbpactor_sumoner_mount)
    (set `self.HoneyValue` 0.0)))

(fn `UserConstructionScript`
  (`parent.UserConstructionScript`))