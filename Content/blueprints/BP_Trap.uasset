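; BP_Trap is a bee trap actor that captures a single bee and then flags bees that enter its second trigger.
; When a bee's SomeSadBox overlaps Box, it checks the class against six bee variants, stores it in BeeInfo, destroys the bee and sets BeeReady.
; While BeeReady, Box1 overlaps set BoolTrap on the bee and point its ActorTrap at itself.
; BeeReady never resets here, and the BeeTrap animation is unwired.
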(event `self.Box.OnComponentBeginOverlap`
  (params (OverlappedComponent :type "PrimitiveComponent Object Reference") (OtherActor :type "Actor Object Reference") (OtherComp :type "PrimitiveComponent Object Reference") (OtherBodyIndex :type Integer) (bFromSweep :type Boolean) (SweepResult :type "HitResult Structure (by ref)"))
  (bind _returnvalue (`GameplayStatics.GetObjectClass` OtherActor))
  (`KismetSystemLibrary.PrintString` (`KismetSystemLibrary.GetDisplayName` OtherComp))
  (bind _asbpchar_bee (cast `/Game/blueprints/bpchar_bee` OtherActor))
  (if (== OtherComp (`/Game/blueprints/bpchar_bee.some_sad_box` _asbpchar_bee))
    (`KismetSystemLibrary.PrintString` "Hello" true true (struct :`R` 1.0 :`G` 0.850331 :`A` 1.0))
    (if (or (== _returnvalue "/Game/blueprints/bpchar_bee.bpchar_bee_C") (== _returnvalue "/Game/blueprints/bpchar_bee_cat.bpchar_bee_cat_C") (== _returnvalue "/Game/blueprints/bpchar_bee_ice.bpchar_bee_ice_C") (== _returnvalue "/Game/blueprints/bpchar_bee_jungke.bpchar_bee_jungke_C") (== _returnvalue "/Game/blueprints/bpchar_bee_rock.bpchar_bee_rock_C") (== _returnvalue "/Game/blueprints/BPchar_lava_bee.BPchar_lava_bee_C"))
      (if (not (`self.Bee Ready?`))
        (bind _output_get (set `self.BeeInfo` (`GameplayStatics.GetObjectClass` OtherActor)))
        (`KismetSystemLibrary.PrintString` (`KismetSystemLibrary.GetClassDisplayName` _output_get) true true (struct :`R` 1.0 :`G` 0.850331 :`A` 1.0))
        (`self.K2_DestroyActor` OtherActor)
        (set `self.Bee Ready?` true)))))

(event `self.Box1.OnComponentBeginOverlap`
  (params (OverlappedComponent :type "PrimitiveComponent Object Reference") (OtherActor :type "Actor Object Reference") (OtherComp :type "PrimitiveComponent Object Reference") (OtherBodyIndex :type Integer) (bFromSweep :type Boolean) (SweepResult :type "HitResult Structure (by ref)"))
  (if (`self.Bee Ready?`)
    (bind _asbpchar_bee (cast `/Game/blueprints/bpchar_bee` OtherActor))
    (set `/Game/blueprints/bpchar_bee.actor_trap` _asbpchar_bee _asbpchar_bee)
    (set `/Game/blueprints/bpchar_bee.bool_trap` true _asbpchar_bee)))

(fn `UserConstructionScript`)