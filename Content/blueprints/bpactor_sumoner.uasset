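; Summoner actor that periodically spawns an instance of its bee class near its own location.
; Tick accumulates elapsed time until it passes the current spawn delay, then resets the timer and picks a new random delay of 30 to 60 seconds.
; Each spawn lands on a random reachable navigation point within a small radius of the root component, with no limit on the number spawned.
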(event `self.ReceiveTick`
  (params (DeltaSeconds :type "Float (single-precision)"))
  (bind _output_get (set `self.float_time` (+ (`self.float_time`) DeltaSeconds)))
  (if (> _output_get (`self.time_for_spawn`))
    (set `self.float_time` 0.0)
    (set `self.time_for_spawn` (`KismetMathLibrary.RandomIntegerInRange` 30 60))
    (`|SpawnActorFromClass` (`self.class_of_bee`) (`KismetMathLibrary.MakeTransform` (`NavigationSystemV1.K2_GetRandomReachablePointInRadius` (`SceneComponent.K2_GetComponentLocation` (`self.DefaultSceneRoot`)) 200.0 null null)) "Undefined" "MultiplyWithRoot" null null)))

(fn `UserConstructionScript`)