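; Lava bee character, a bee variant that harms its surroundings and delivers honey to the lava summoner.
; Sphere1 tracks the player, and a looping one-second timer calls FireX on them while inside.
; Each tick it destroys non-lava bees overlapping that sphere.
; When its Box touches a lava summoner, it adds its scaled HoneyValue to the summoner's Honey and resets its own to zero.
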(event `self.ReceiveBeginPlay`
  (`parent.ReceiveBeginPlay`)
  (`KismetSystemLibrary.K2_SetTimerDelegate` (delegate `What?`) 1.0 true))

(event `What?`
  (if (`self.?`)
    (bind _asbp_first_person_character (cast `/Game/FirstPerson/Blueprints/BP_FirstPersonCharacter` (`GameplayStatics.GetPlayerPawn` 0)))
    (`/Game/FirstPerson/Blueprints/BP_FirstPersonCharacter.FireX` _asbp_first_person_character)))

(event `self.ReceiveActorBeginOverlap`
  (params (OtherActor :type "Actor Object Reference"))
  (`parent.ReceiveActorBeginOverlap` OtherActor))

(event `self.ReceiveTick`
  (params (DeltaSeconds :type "Float (single-precision)"))
  (`parent.ReceiveTick` DeltaSeconds)
  (for _array_element (`PrimitiveComponent.GetOverlappingActors` (`self.Sphere1`) "/Game/blueprints/bpchar_bee.bpchar_bee_C")
    (if (!= (`GameplayStatics.GetObjectClass` _array_element) "BPchar_lava_bee_C")
      (`self.K2_DestroyActor` _array_element))))

(event `self.Sphere1.OnComponentBeginOverlap`
  (params (OverlappedComponent :type "PrimitiveComponent Object Reference") (OtherActor :type "Actor Object Reference") (OtherComp :type "PrimitiveComponent Object Reference") (OtherBodyIndex :type Integer) (bFromSweep :type Boolean) (SweepResult :type "HitResult Structure (by ref)"))
  (if (== OtherActor (`GameplayStatics.GetPlayerPawn` 0))
    (set `self.?` true)))

(event `self.Sphere1.OnComponentEndOverlap`
  (params (OverlappedComponent :type "PrimitiveComponent Object Reference") (OtherActor :type "Actor Object Reference") (OtherComp :type "PrimitiveComponent Object Reference") (OtherBodyIndex :type Integer))
  (if (== OtherActor (`GameplayStatics.GetPlayerPawn` 0))
    (set `self.?` false)))

(event `self.Box.OnComponentBeginOverlap`
  (params (OverlappedComponent :type "PrimitiveComponent Object Reference") (OtherActor :type "Actor Object Reference") (OtherComp :type "PrimitiveComponent Object Reference") (OtherBodyIndex :type Integer) (bFromSweep :type Boolean) (SweepResult :type "HitResult Structure (by ref)"))
  (if (== (`GameplayStatics.GetObjectClass` OtherActor) "/Game/blueprints/bpac_sumoner/bpactor_sumoner_LAVA.bpactor_sumoner_LAVA_C")
    (bind _asbpactor_sumoner_lava (cast `/Game/blueprints/bpac_sumoner/bpactor_sumoner_LAVA` OtherActor))
    (set `/Game/blueprints/bpac_sumoner/bpactor_sumoner.Honey` (+ (`/Game/blueprints/bpac_sumoner/bpactor_sumoner.Honey` _asbpactor_sumoner_lava) (/ (`self.HoneyValue`) 100.0)) _asbpactor_sumoner_lava)
    (set `self.HoneyValue` 0.0)))

(fn `UserConstructionScript`
  (`parent.UserConstructionScript`))